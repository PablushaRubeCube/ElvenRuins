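; BP_Door is a door that slides along Z once enough open requests have been received.
; OpenDoor and CloseDoor raise and lower a counter; reaching RequirementCount exactly plays a rock-moving sound and the Door timeline.
; The timeline's DoorTrack offsets the static mesh from its location saved at BeginPlay.
; When SwitchCloseDoor is set, any CloseDoor call leaving the count below the requirement replays the sound and reverses the timeline.
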(event EventBeginPlay
  (Variables|Default|SetInitialLocation (Transformation|GetWorldLocation (Variables|Default|GetStaticMesh))))

(event EventOpenDoor
  (bind _initiallocation (Variables|Default|GetInitialLocation))
  (Math|Integer|IncrementInt (Variables|Default|GetCountOpenDoor)
    (:%20%20
      (if (== (Variables|Default|GetRequirementCount) (Variables|Default|GetCountOpenDoor))
        (Audio|PlaySound2D "/Game/Lesson/Sounds/zapsplat_foley_large_rock_movement_006_13471__1__Cue.zapsplat_foley_large_rock_movement_006_13471__1__Cue" 1.0 1.0 0.0 0 0)
        (bind _doortrack (Timeline|Door Play)
          (:Update
            (Transformation|SetWorldLocation (Variables|Default|GetStaticMesh) (Math|Vector|MakeVector (.x _initiallocation) (.y _initiallocation) (+ (.z _initiallocation) _doortrack)) false false)))))))

(event EventCloseDoor
  (bind _initiallocation (Variables|Default|GetInitialLocation))
  (Math|Integer|DecrementInt (Variables|Default|GetCountOpenDoor)
    (:%20%20
      (if (and (< (Variables|Default|GetCountOpenDoor) (Variables|Default|GetRequirementCount)) (Variables|Default|GetSwitchCloseDoor))
        (Audio|PlaySound2D "/Game/Lesson/Sounds/zapsplat_foley_large_rock_movement_006_13471__1__Cue.zapsplat_foley_large_rock_movement_006_13471__1__Cue" 1.0 1.0 0.0 0 0)
        (bind _doortrack (Timeline|Door Reverse)
          (:Update
            (Transformation|SetWorldLocation (Variables|Default|GetStaticMesh) (Math|Vector|MakeVector (.x _initiallocation) (.y _initiallocation) (+ (.z _initiallocation) _doortrack)) false false)))))))

(fn ConstructionScript)