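; BP_Statue is a puzzle-driven statue whose Fountain component rises and rotates once enough OpenDoor signals arrive.
; OpenDoor and CloseDoor adjust a counter, playing the Door timeline when it equals RequirementCount and reversing it on any close that leaves it below.
; The timeline drives Z offset and yaw from the transform cached at BeginPlay, with a rock-movement sound on each play or reverse.
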(event EventBeginPlay
  (bind _fountain (Variables|Default|GetFountain))
  (Variables|Default|SetInitialLocation (Transformation|GetWorldLocation _fountain))
  (Variables|Default|SetInitialRotation (Transformation|GetWorldRotation _fountain)))

(event EventOpenDoor
  (bind _initiallocation (Variables|Default|GetInitialLocation))
  (bind _initialrotation (Variables|Default|GetInitialRotation))
  (Math|Integer|IncrementInt (Variables|Default|GetCountOpenDoor)
    (:%20%20
      (if (== (Variables|Default|GetRequirementCount) (Variables|Default|GetCountOpenDoor))
        (Audio|PlaySound2D "/Game/Lesson/Sounds/zapsplat_foley_large_rock_movement_006_13471__1__Cue.zapsplat_foley_large_rock_movement_006_13471__1__Cue" 1.0 1.0 0.0 0 0)
        (bind (_direction _fountaintrack _rotationangel) (Timeline|Door Play)
          (:Update
            (Transformation|SetWorldLocationAndRotation (Variables|Default|GetFountain) (Math|Vector|MakeVector (.x _initiallocation) (.y _initiallocation) (+ (.z _initiallocation) _fountaintrack)) (Math|Rotator|MakeRotator (.roll _initialrotation) (.pitch _initialrotation) (+ _rotationangel (.yaw _initialrotation))) false false)))))))

(event EventCloseDoor
  (bind _initiallocation (Variables|Default|GetInitialLocation))
  (bind _initialrotation (Variables|Default|GetInitialRotation))
  (Math|Integer|DecrementInt (Variables|Default|GetCountOpenDoor)
    (:%20%20
      (if (< (Variables|Default|GetCountOpenDoor) (Variables|Default|GetRequirementCount))
        (Audio|PlaySound2D "/Game/Lesson/Sounds/zapsplat_foley_large_rock_movement_006_13471__1__Cue.zapsplat_foley_large_rock_movement_006_13471__1__Cue" 1.0 1.0 0.0 0 0)
        (bind (_direction _fountaintrack _rotationangel) (Timeline|Door Reverse)
          (:Update
            (Transformation|SetWorldLocationAndRotation (Variables|Default|GetFountain) (Math|Vector|MakeVector (.x _initiallocation) (.y _initiallocation) (+ (.z _initiallocation) _fountaintrack)) (Math|Rotator|MakeRotator (.roll _initialrotation) (.pitch _initialrotation) (+ _rotationangel (.yaw _initialrotation))) false false)))))))

(fn ConstructionScript)