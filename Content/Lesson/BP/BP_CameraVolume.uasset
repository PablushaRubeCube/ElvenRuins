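; Camera volume that becomes the player's view when a PuzzleCharacter enters its Box.
; On overlap it registers itself on the character and PuzzleController as the current camera, then eases the view target over to itself.
; With UseSpline enabled, Tick smoothly moves the Camera to the Spline point closest to that character and turns it to face them.
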(event OnComponentBeginOverlap(Box)
  (params (OverlappedComponent :type Primitive%20Component%20Object%20Reference) (OtherActor :type Actor%20Object%20Reference) (OtherComp :type Primitive%20Component%20Object%20Reference) (OtherBodyIndex :type Integer) (bFromSweep :type Boolean) (SweepResult :type Hit%20Result%20Structure%20%28by%20ref%29))
  (bind _self self)
  (bind _refcontroller (Variables|Default|GetRefController))
  (bind _aspuzzle_character (Utilities|Casting|CastToPuzzleCharacter OtherActor))
  (bind _output_get (Variables|Default|SetAs%20Puzzle%20Character _aspuzzle_character))
  (Utilities|IsValid _refcontroller
    (:Is%20Valid
      (Variables|/Game/Lesson/BP/Character/PuzzleCharacter.PuzzleCharacter_C|SetCameraVolume _output_get _self)
      (Variables|/Game/Lesson/BP/PuzzleController.PuzzleController_C|SetCurrentCamera (.AsPuzzle%20Controller (Utilities|Casting|CastToPuzzleController (Variables|Default|GetRefController))) _self)
      (Game|Player|SetViewTargetwithBlend _refcontroller _self 2.0 "VTBlend_EaseInOut" 3.0 true))))

(event EventBeginPlay
  (Variables|Default|SetRefController (Game|GetPlayerController 0))
  (Variables|Default|SetSplineOn? (Variables|Camera|GetUseSpline)))

(event EventTick
  (params (DeltaSeconds :type Float%20%28single-precision%29))
  (bind _as_puzzle_character (Variables|Default|GetAs%20Puzzle%20Character))
  (bind _camera (Variables|Default|GetCamera))
  (bind _returnvalue (Transformation|GetActorLocation _as_puzzle_character))
  (Variables|Default|SetDelta%20Seconds DeltaSeconds)
  (if (Variables|Camera|GetUseSpline)
    (Utilities|IsValid (Variables|Default|GetAs%20Puzzle%20Character)
      (:Is%20Valid
        (Transformation|SetWorldLocationAndRotation (Variables|Default|GetCamera) (Math|Interpolation|VInterpTo (Transformation|GetWorldLocation _camera) (Spline|FindLocationClosesttoWorldLocation (Variables|Default|GetSpline) _returnvalue "World") (Variables|Default|GetDelta%20Seconds) 2.0) (Math|Interpolation|RInterpTo (Transformation|GetWorldRotation _camera) (Math|Rotator|FindLookatRotation (Transformation|GetWorldLocation (Variables|Default|GetCamera)) _returnvalue) (Variables|Default|GetDelta%20Seconds) 2.0) false false)))))

(fn ConstructionScript)